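; BP_GGJCharacter is a flipbook-based 2D character whose identity can be swapped at runtime.
; ChangeCharacterIdentity validates the supplied flipbooks and anim instance class, then applies them to the body Sprite, the separate MaskSprite and the AnimationComponent.
; It stores the new CharacterID and returns true on success, or changes nothing and returns false if any asset is invalid.
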(fn ConstructionScript)

(fn ChangeCharacterIdentity
  (params (CharacterID :type Integer) (CharacterFlipbook :type Paper%20Flipbook%20Object%20Reference) (MaskFlipbook :type Paper%20Flipbook%20Object%20Reference) (AnimInstance :type Paper%20ZD%20Anim%20Instance%20Class%20Reference))
  (if (Math|Boolean|ANDBoolean (Utilities|IsValid CharacterFlipbook) (Utilities|IsValidClass AnimInstance) (Utilities|IsValid MaskFlipbook))
    (Sprite|SetFlipbook (Variables|Default|GetSprite) CharacterFlipbook)
    (Sprite|SetFlipbook (Variables|Default|GetMaskSprite) MaskFlipbook)
    (Class|PaperZDAnimationComponent|SetAnimInstanceClass (Variables|Default|GetAnimationComponent) AnimInstance)
    (Variables|Default|SetCharacterID CharacterID)
    (return true)
    (else
      (return false))))
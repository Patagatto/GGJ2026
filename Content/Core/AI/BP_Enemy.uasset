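; BP_Enemy is an AI enemy Blueprint whose graph handles hit and death audio feedback.
; On begin play it starts the player attack-hit MetaSound on its Audio component.
; Each hit reads player 0's attack combo index, prints it, passes it as the sound's Index parameter and fires its trigger, so audio follows the combo.
; On death, the MSSPlayerAttackHit component switches to the death sound and plays it.
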(event EventOnEnemyHit
  (bind _audio (Variables|Default|GetAudio))
  (bind _asbp_ggjcharacter (Utilities|Casting|CastToBP_GGJCharacter (Game|Player|GetPlayerPawn 0)))
  (Development|PrintString (Utilities|String|ToString(Integer) (Variables|/Script/GGJ2026.GGJCharacter|GetAttackComboIndex _asbp_ggjcharacter)))
  (Effects|Components|ParticleSystem|SetIntParameter _audio "Index" (Variables|/Script/GGJ2026.GGJCharacter|GetAttackComboIndex _asbp_ggjcharacter))
  (Class|AudioParameterControllerInterface|SetTriggerParameter _audio "In"))

(event EventOnEnemyDied
  (bind _mss_playerattackhit (Variables|Default|GetMSS_PlayerAttackHit))
  (Audio|Components|Audio|SetSound _mss_playerattackhit "/Game/Assets/Sound/SFX/PlayerDeath/MSS_Death.MSS_Death")
  (Audio|Components|Audio|Play _mss_playerattackhit 0.0))

(event EventBeginPlay
  (bind _audio (Variables|Default|GetAudio))
  (Audio|Components|Audio|SetSound _audio "/Game/Assets/Sound/SFX/PlayerAttack/Hit/MSS_PlayerAttackHit.MSS_PlayerAttackHit")
  (Audio|Components|Audio|Play _audio 0.0))

(fn ConstructionScript)
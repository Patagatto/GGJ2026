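; BP_GGJCharacterTest is a flipbook-based test character with a roll action and a swappable identity.
; The roll input sets ActionState to Rolling, then resets it to None after a short delay.
; ChangeCharacterIdentity validates its assets, then swaps the body and mask flipbooks and the AnimationComponent's anim instance class, stores the CharacterID and returns whether it succeeded.
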(event Input|EnhancedActionEvents|EnhancedInputActionIA_Roll
  (params (ActionValue :type Boolean) (ElapsedSeconds :type Float%20%28double-precision%29) (TriggeredSeconds :type Float%20%28double-precision%29) (InputAction :type Input%20Action%20Object%20Reference :default "/Game/Core/Input/InputAction/IA_Roll.IA_Roll"))
  (:Started
    (Variables|Default|SetActionState "Rolling")
    (Utilities|FlowControl|Delay 0.1)
    (Variables|Default|SetActionState "None")))

(event EventBeginPlay)

(event Collision|EventActorBeginOverlap
  (params (OtherActor :type Actor%20Object%20Reference)))

(event EventTick
  (params (DeltaSeconds :type Float%20%28single-precision%29)))

(fn ConstructionScript)

(fn ChangeCharacterIdentity
  (params (CharacterID :type Integer) (CharacterFlipbook :type Paper%20Flipbook%20Object%20Reference) (MaskFlipbook :type Paper%20Flipbook%20Object%20Reference) (AnimInstance :type Paper%20ZD%20Anim%20Instance%20Class%20Reference))
  (if (Math|Boolean|ANDBoolean (Utilities|IsValid CharacterFlipbook) (Utilities|IsValidClass AnimInstance) (Utilities|IsValid MaskFlipbook))
    (Sprite|SetFlipbook (Variables|Default|GetSprite) CharacterFlipbook)
    (Sprite|SetFlipbook (Variables|Default|GetMaskSprite) MaskFlipbook)
    (Class|PaperZDAnimationComponent|SetAnimInstanceClass (Variables|Default|GetAnimationComponent) AnimInstance)
    (Variables|Default|SetCharacterID CharacterID)
    (return true)
    (else
      (return false))))
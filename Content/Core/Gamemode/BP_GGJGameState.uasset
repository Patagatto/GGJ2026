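; Game state that assigns social relationships between all generated NPC characters when play begins.
; MakeRelationship shuffles the NPCs with a millisecond-seeded random stream, numbers them by index, then fills each one's MapRelations for every other NPC.
; The first two shuffled IDs receive a different relation type from the rest, in everyone else's map.
; GetSocialStatus is a stub returning a constant, with its lover and hater lookups disconnected.
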(event EventBeginPlay
  (Variables|Default|SetRandomStream (Math|Random|MakeRandomStream (Math|DateTime|GetMillisecond (Math|DateTime|Now))))
  (CallFunction|MakeRelationship))

(event EventTick
  (params (DeltaSeconds :type Float%20%28single-precision%29)))

(fn ConstructionScript)

(fn MakeRelationship
  (Utilities|Array|Clear (LocalVariables|GetTempIDList))
  (Utilities|Array|Clear (LocalVariables|GetAllNpcs))
  (bind _outactors (Actor|GetAllActorsOfClass "/Game/Testing/BP_GeneratedCharacter.BP_GeneratedCharacter_C"))
  (bind _output_get (LocalVariables|SetAllNpcs _outactors))
  (Utilities|Array|ShuffleFromStream _output_get (Variables|Default|GetRandomStream))
  (for (_array_element _array_index) (LocalVariables|GetAllNpcs)
    (Variables|/Game/Testing/BP_GeneratedCharacter.BP_GeneratedCharacter_C|SetNPCID _array_element _array_index)
    (Utilities|Map|Clear (Variables|/Game/Testing/BP_GeneratedCharacter.BP_GeneratedCharacter_C|GetMapRelations _array_element)))
  (for _array_element_2 (LocalVariables|GetAllNpcs)
    (Utilities|Array|Clear (LocalVariables|GetTempIDList))
    (for (_array_element_3 _array_index_2) (LocalVariables|GetAllNpcs)
      (if (!= (Variables|/Game/Testing/BP_GeneratedCharacter.BP_GeneratedCharacter_C|GetNPCID _array_element_2) _array_index_2)
        (Utilities|Array|AddUnique (LocalVariables|GetTempIDList) (Variables|/Game/Testing/BP_GeneratedCharacter.BP_GeneratedCharacter_C|GetNPCID _array_element_3))))
    (Utilities|Array|ShuffleFromStream (LocalVariables|GetTempIDList) (Variables|Default|GetRandomStream))
    (for _index (range 0 (Utilities|Array|LastIndex (LocalVariables|GetTempIDList)))
      (bind _output_get_2 (LocalVariables|SetTargetID (Utilities|Array|Get(acopy) (LocalVariables|GetTempIDList) _index)))
      (if (< _output_get_2 2)
        (Utilities|Map|Add (Variables|/Game/Testing/BP_GeneratedCharacter.BP_GeneratedCharacter_C|GetMapRelations _array_element_2) _output_get_2 "NewEnumerator2")
        (else
          (Utilities|Map|Add (Variables|/Game/Testing/BP_GeneratedCharacter.BP_GeneratedCharacter_C|GetMapRelations _array_element_2) _output_get_2 "NewEnumerator0"))))))

(fn GetSocialStatus
  (params (WatcherID :type Integer) (TargetID :type Integer))
  (if true
    (return "NewEnumerator2")
    (elif true
      (return "NewEnumerator0"))))
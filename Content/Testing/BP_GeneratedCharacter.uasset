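; BP_GeneratedCharacter is a randomized masked NPC, in a testing folder, that can report whom it likes and hates.
; BeginPlay randomizes body gender, mask and mask color from arrays and maps, then displays Name, which is built from those labels only on the female branch.
; Box overlap prints relationships looked up by NPCID in BP_GGJGameState's lover and hater maps, using a DoOnce reset on end overlap.
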(event OnComponentBeginOverlap(Box)
  (params (OverlappedComponent :type Primitive%20Component%20Object%20Reference) (OtherActor :type Actor%20Object%20Reference) (OtherComp :type Primitive%20Component%20Object%20Reference) (OtherBodyIndex :type Integer) (bFromSweep :type Boolean) (SweepResult :type Hit%20Result%20Structure%20%28by%20ref%29))
  (bind _npcid (Variables|NPCID|GetNPCID))
  (bind _npcid_2 (Variables|NPCID|GetNPCID))
  (Utilities|FlowControl|DoOnce false
    (:Completed
      (bind _asbp_ggjgame_state (Utilities|Casting|CastToBP_GGJGameState (Game|GetGameState)))
      (Development|PrintString (Utilities|String|ToString(Text) (Utilities|Text|FormatText "{Name} likes {Targets}" _npcid (.Value (Utilities|Map|Find (Variables|/Game/Core/Gamemode/BP_GGJGameState.BP_GGJGameState_C|GetMapLovers _asbp_ggjgame_state) _npcid)))) true true "(R=0.000000,G=0.660000,B=1.000000,A=1.000000)" 3.0)
      (Development|PrintString (Utilities|String|ToString(Text) (Utilities|Text|FormatText "{Name} Hate {Targets}" _npcid_2 (.Value (Utilities|Map|Find (Variables|/Game/Core/Gamemode/BP_GGJGameState.BP_GGJGameState_C|GetMapHaters _asbp_ggjgame_state) _npcid_2))))))))

(event OnComponentEndOverlap(Box)
  (params (OverlappedComponent :type Primitive%20Component%20Object%20Reference) (OtherActor :type Actor%20Object%20Reference) (OtherComp :type Primitive%20Component%20Object%20Reference) (OtherBodyIndex :type Integer))
  (bind _npcid (Variables|NPCID|GetNPCID))
  (bind _npcid_2 (Variables|NPCID|GetNPCID))
  (Utilities|FlowControl|DoOnce false) ; enters at Reset
)

(event EventBeginPlay
  ;[0.15 0.15 0.15 0.5] 0=Male, 1=Female
  (Variables|Default|SetFemale (Math|Random|RandomBool))
  (Rendering|Components|Sprite|SetSprite (Variables|Default|GetBody) (Utilities|Array|Get(acopy) (Variables|Default|GetBodyArray) (Math|Conversions|ToInteger(Boolean) (Variables|Default|GetFemale))))
  ;[0.15 0.15 0.15 0.5] 0=CatMask, 1=PeacockMask, 2=RabbitMask
  (Variables|Default|SetMaskIndex (Math|Random|RandomInteger 3))
  (Rendering|Components|Sprite|SetSprite (Variables|Default|GetMask) (.Key (Utilities|Map|GetKeyValueByIndex (Variables|Default|GetMaskArray) (Variables|Default|GetMaskIndex))))
  ;[0.15 0.15 0.15 0.5] Color Definition
  (Variables|Default|SetColorIndex (Math|Random|RandomInteger 3))
  (Sprite|SetSpriteColor (Variables|Default|GetMask) (.Key (Utilities|Map|GetKeyValueByIndex (Variables|Default|GetColorArray) (Variables|Default|GetColorIndex))))
  ;[0.15 0.15 0.15 0.5] Set Text Name
  (if (Variables|Default|GetFemale)
    (Variables|Default|SetGender "Ms.")
    (bind _output_get (Variables|Default|SetName (Utilities|Text|FormatText "{Gender} {Color} {Mask}" (Variables|Default|GetGender) (.Value (Utilities|Map|GetKeyValueByIndex (Variables|Default|GetColorArray) (Variables|Default|GetColorIndex))) (.Value (Utilities|Map|GetKeyValueByIndex (Variables|Default|GetMaskArray) (Variables|Default|GetMaskIndex))))))
    (else
      (Variables|Default|SetGender "Mr.")))
  (Rendering|Components|TextRender|SetText (Variables|Default|GetTextRender) _output_get))

(event Collision|EventActorBeginOverlap
  (params (OtherActor :type Actor%20Object%20Reference)))

(event EventTick
  (params (DeltaSeconds :type Float%20%28single-precision%29)))

(fn ConstructionScript)
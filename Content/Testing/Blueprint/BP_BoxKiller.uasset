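; BP_BoxKiller is a test trigger actor that makes an overlapping player character take over the identity of the nearest generated NPC.
; On the first Box overlap, gated by DoOnce, it casts to BP_GGJCharacter and finds the closest BP_GeneratedCharacter.
; It calls ChangeCharacterIdentity with that NPC's ID and a hardcoded chandelier flipbook, then destroys the nearest NPC.
; Debug prints show the character ID before and after the swap.
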(event OnComponentBeginOverlap(Box)
  (params (OverlappedComponent :type Primitive%20Component%20Object%20Reference) (OtherActor :type Actor%20Object%20Reference) (OtherComp :type Primitive%20Component%20Object%20Reference) (OtherBodyIndex :type Integer) (bFromSweep :type Boolean) (SweepResult :type Hit%20Result%20Structure%20%28by%20ref%29))
  (Utilities|FlowControl|DoOnce false
    (:Completed
      (bind _asbp_ggjcharacter (Utilities|Casting|CastToBP_GGJCharacter OtherActor))
      (Development|PrintString (Utilities|String|ToString(Integer) (Variables|/Game/Core/Characters/BP_GGJCharacter.BP_GGJCharacter_C|GetCharacterID _asbp_ggjcharacter)))
      (bind _outactors (Actor|GetAllActorsOfClass "/Game/Testing/BP_GeneratedCharacter.BP_GeneratedCharacter_C"))
      (bind _asbp_generated_character (Utilities|Casting|CastToBP_GeneratedCharacter (.ReturnValue (Actor|FindNearestActor (Transformation|GetActorLocation _asbp_ggjcharacter) _outactors))))
      (Default|ChangeCharacterIdentity _asbp_ggjcharacter (Variables|/Game/Testing/BP_GeneratedCharacter.BP_GeneratedCharacter_C|GetNPCID _asbp_generated_character) "/Game/Testing/Sprite/EnviroementAssets/Chandelier/Sprites/FB_Chandelier.FB_Chandelier" "/Script/PaperZD.PaperZDAnimInstance")
      (Development|PrintString (Utilities|String|ToString(Integer) (Variables|/Game/Core/Characters/BP_GGJCharacter.BP_GGJCharacter_C|GetCharacterID _asbp_ggjcharacter)))
      (Actor|DestroyActor (.ReturnValue (Actor|FindNearestActor (Transformation|GetActorLocation _asbp_ggjcharacter) _outactors))))))

(event EventBeginPlay)

(event Collision|EventActorBeginOverlap
  (params (OtherActor :type Actor%20Object%20Reference)))

(event EventTick
  (params (DeltaSeconds :type Float%20%28single-precision%29)))

(fn ConstructionScript)